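; BP_Heal_kit is a single-use healing pickup.
; When the ThirdPersonCharacter overlaps its Box, it calls HealthAdd with PickupAmount, plays a sound at its location and destroys itself.
; On BeginPlay it writes PickupAmount into the Amount text and points RotatingMovement at SceneComponentHealthAmount, so only that health amount component is rotated by the movement component.
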(event OnComponentBeginOverlap(Box)
  (params (OverlappedComponent :type Primitive%20Component%20Object%20Reference) (OtherActor :type Actor%20Object%20Reference) (OtherComp :type Primitive%20Component%20Object%20Reference) (OtherBodyIndex :type Integer) (bFromSweep :type Boolean) (SweepResult :type Hit%20Result%20Structure%20%28by%20ref%29))
  ;[1 1 1] Kertakäyttöisyys esineelle
  (bind _asthird_person_character (Utilities|Casting|CastToThirdPersonCharacter OtherActor))
  (Default|HealthAdd _asthird_person_character (Variables|Default|GetPickupAmount))
  (Audio|PlaySoundatLocation "/Game/ASSETIT/SOUNDS/Mushroom_1_by_StarNinjas_Cue.Mushroom_1_by_StarNinjas_Cue" (Transformation|GetActorLocation) "0, 0, 0" 1.0 1.0 0.0 0 0 0)
  (Actor|DestroyActor))

(event EventBeginPlay
  ;[1 1 1] Parannuksen määrän näyttäminen ja pyöriminen
  (Rendering|Components|TextRender|SetText (Variables|Default|GetAmount) (Utilities|Text|ToText(Integer) (Variables|Default|GetPickupAmount)))
  (Components|Movement|SetUpdatedComponent (Variables|Default|GetRotatingMovement) (Variables|Default|GetScene%20Component%20Health%20amount)))

(fn ConstructionScript)