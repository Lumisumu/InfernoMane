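; Music manager that switches between level tracks and the player character's battle music.
; BeginPlay starts every TrackList song muted and unmutes the starting one, so switches only change volume.
; ChangeMusicTo rechecks detection and combat music after a retriggerable delay, only storing the requested track during combat for later resumption.
; Battle and boss events mute or restore that track while fading the character's BattleMusic; boss events never play BossMusic.
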(event Custom|ChangeMusicTo
  (params (IndexOfSongToPlay :type Integer) (Actor :type Actor%20Object%20Reference))
  (bind _musicrefs (Variables|Default|GetMusicRefs))
  (bind _output (Utilities|Array|Get(acopy) _musicrefs IndexOfSongToPlay))
  ;[1 1 1] Changes the current music to whichever index is given, unless the unicorn is being detected by an enemy, then it keeps the battle music which should be going on, and updates the next song into the current reference for later
  (bind _asthird_person_character (Utilities|Casting|CastToThirdPersonCharacter Actor))
  (if (Math|Boolean|ORBoolean (Variables|/Game/ThirdPersonBP/Blueprints/ThirdPersonCharacter.ThirdPersonCharacter_C|GetIsDetected _asthird_person_character) (!= (Variables|/Script/Engine.AudioComponent|GetVolumeMultiplier (Variables|/Game/ThirdPersonBP/Blueprints/ThirdPersonCharacter.ThirdPersonCharacter_C|GetBattleMusic _asthird_person_character)) 0.0) (!= 0.0 (Variables|/Script/Engine.AudioComponent|GetVolumeMultiplier (Variables|/Game/ThirdPersonBP/Blueprints/ThirdPersonCharacter.ThirdPersonCharacter_C|GetBossMusic _asthird_person_character))))
    (Variables|Default|SetCurrentMusicRef (Utilities|Array|Get(acopy) (Variables|Default|GetMusicRefs) IndexOfSongToPlay) :!label _label)
    (else
      (Utilities|FlowControl|RetriggerableDelay 1.0)
      (if (Math|Boolean|ORBoolean (Variables|/Game/ThirdPersonBP/Blueprints/ThirdPersonCharacter.ThirdPersonCharacter_C|GetIsDetected _asthird_person_character) (!= (Variables|/Script/Engine.AudioComponent|GetVolumeMultiplier (Variables|/Game/ThirdPersonBP/Blueprints/ThirdPersonCharacter.ThirdPersonCharacter_C|GetBattleMusic _asthird_person_character)) 0.0) (!= 0.0 (Variables|/Script/Engine.AudioComponent|GetVolumeMultiplier (Variables|/Game/ThirdPersonBP/Blueprints/ThirdPersonCharacter.ThirdPersonCharacter_C|GetBossMusic _asthird_person_character))))
        (goto _label)
        (else
          (Audio|Components|Audio|SetVolumeMultiplier (Variables|Default|GetCurrentMusicRef) 0.0 :!class /Script/Engine.AudioComponent)
          (Audio|Components|Audio|SetVolumeMultiplier _output 1.0 :!class /Script/Engine.AudioComponent)
          (Variables|Default|SetCurrentMusicRef _output))))))

(event Custom|BossMusicOFF
  (params (BattleMusicIndex :type Integer) (Pelaaja :type Actor%20Object%20Reference))
  (bind _currentmusicref (Variables|Default|GetCurrentMusicRef))
  ;[1 1 1] Changes boss music volume to 0 and previous music volume to 1
  (bind _asthird_person_character (Utilities|Casting|CastToThirdPersonCharacter Pelaaja))
  (Variables|/Game/ThirdPersonBP/Blueprints/ThirdPersonCharacter.ThirdPersonCharacter_C|SetBattleMusicEnding _asthird_person_character true)
  (Audio|Components|Audio|FadeOut (Variables|/Game/ThirdPersonBP/Blueprints/ThirdPersonCharacter.ThirdPersonCharacter_C|GetBattleMusic _asthird_person_character) 2.0 0.0 "Linear" :!class /Script/Engine.AudioComponent)
  (Utilities|FlowControl|Delay 2.0)
  (Audio|Components|Audio|SetVolumeMultiplier (Variables|/Game/ThirdPersonBP/Blueprints/ThirdPersonCharacter.ThirdPersonCharacter_C|GetBattleMusic _asthird_person_character) 0.0 :!class /Script/Engine.AudioComponent)
  (Variables|/Game/ThirdPersonBP/Blueprints/ThirdPersonCharacter.ThirdPersonCharacter_C|SetBattleMusicEnding _asthird_person_character false)
  (Audio|Components|Audio|SetVolumeMultiplier _currentmusicref 1.0 :!class /Script/Engine.AudioComponent)
  (Audio|Components|Audio|AdjustVolume _currentmusicref 1.0 (Variables|Default|GetMusicVolume) "Linear" :!class /Script/Engine.AudioComponent))

(event Custom|BossMusicON
  (params (BattleMusicIndex :type Integer) (Pelaaja :type Actor%20Object%20Reference))
  (bind _currentmusicref (Variables|Default|GetCurrentMusicRef))
  ;[1 1 1] Changes boss music volume to 1 and previous music to 0
  (Audio|Components|Audio|AdjustVolume _currentmusicref 1.0 0.0 "Linear" :!class /Script/Engine.AudioComponent)
  (Audio|Components|Audio|SetVolumeMultiplier _currentmusicref 0.0 :!class /Script/Engine.AudioComponent)
  (bind _asthird_person_character (Utilities|Casting|CastToThirdPersonCharacter Pelaaja))
  (Audio|Components|Audio|SetVolumeMultiplier (Variables|/Game/ThirdPersonBP/Blueprints/ThirdPersonCharacter.ThirdPersonCharacter_C|GetBattleMusic _asthird_person_character) 1.0 :!class /Script/Engine.AudioComponent)
  (Audio|Components|Audio|AdjustVolume (Variables|/Game/ThirdPersonBP/Blueprints/ThirdPersonCharacter.ThirdPersonCharacter_C|GetBattleMusic _asthird_person_character) 0.0 0.0 "Linear" :!class /Script/Engine.AudioComponent)
  (Audio|Components|Audio|FadeIn (Variables|/Game/ThirdPersonBP/Blueprints/ThirdPersonCharacter.ThirdPersonCharacter_C|GetBattleMusic _asthird_person_character) 2.0 (Variables|Default|GetMusicVolume) 0.0 "Linear" :!class /Script/Engine.AudioComponent))

(event Custom|Battle%20Music%20On
  (params (BattleMusicIndex :type Integer) (Pelaaja :type Actor%20Object%20Reference))
  ;[1 1 1] Changes battle music volume to 1 and previous music to 0
  (Audio|Components|Audio|SetVolumeMultiplier (Variables|Default|GetCurrentMusicRef) 0.0 :!class /Script/Engine.AudioComponent)
  (bind _asthird_person_character (Utilities|Casting|CastToThirdPersonCharacter Pelaaja))
  (Audio|Components|Audio|SetVolumeMultiplier (Variables|/Game/ThirdPersonBP/Blueprints/ThirdPersonCharacter.ThirdPersonCharacter_C|GetBattleMusic _asthird_person_character) 1.0 :!class /Script/Engine.AudioComponent)
  (Audio|Components|Audio|AdjustVolume (Variables|/Game/ThirdPersonBP/Blueprints/ThirdPersonCharacter.ThirdPersonCharacter_C|GetBattleMusic _asthird_person_character) 0.0 0.0 "Linear" :!class /Script/Engine.AudioComponent)
  (Audio|Components|Audio|FadeIn (Variables|/Game/ThirdPersonBP/Blueprints/ThirdPersonCharacter.ThirdPersonCharacter_C|GetBattleMusic _asthird_person_character) 2.0 (Variables|Default|GetMusicVolume) 0.0 "Linear" :!class /Script/Engine.AudioComponent))

(event Custom|Battle%20Music%20Off
  (params (BattleMusicIndex :type Integer) (Pelaaja :type Actor%20Object%20Reference))
  ;[1 1 1] Changes battle music volume to 0 and previous music volume to 1
  (bind _asthird_person_character (Utilities|Casting|CastToThirdPersonCharacter Pelaaja))
  (Variables|/Game/ThirdPersonBP/Blueprints/ThirdPersonCharacter.ThirdPersonCharacter_C|SetBattleMusicEnding _asthird_person_character true)
  (Audio|Components|Audio|FadeOut (Variables|/Game/ThirdPersonBP/Blueprints/ThirdPersonCharacter.ThirdPersonCharacter_C|GetBattleMusic _asthird_person_character) 2.0 0.0 "Linear" :!class /Script/Engine.AudioComponent)
  (Utilities|FlowControl|Delay 2.0)
  (Audio|Components|Audio|SetVolumeMultiplier (Variables|/Game/ThirdPersonBP/Blueprints/ThirdPersonCharacter.ThirdPersonCharacter_C|GetBattleMusic _asthird_person_character) 0.0 :!class /Script/Engine.AudioComponent)
  (Variables|/Game/ThirdPersonBP/Blueprints/ThirdPersonCharacter.ThirdPersonCharacter_C|SetBattleMusicEnding _asthird_person_character false)
  (Audio|Components|Audio|SetVolumeMultiplier (Variables|Default|GetCurrentMusicRef) 1.0 :!class /Script/Engine.AudioComponent))

(event EventBeginPlay
  (bind _musicrefs (Variables|Default|GetMusicRefs))
  (bind _indexofsongtoplayonlevelbegin (Variables|Default|GetIndexOfSongToPlayOnLevelBegin))
  (bind _output (Utilities|Array|Get(acopy) _musicrefs _indexofsongtoplayonlevelbegin))
  ;[1 1 1] Plays all of the songs at volume 0 and then the forest ambience track at volume 1
  (for _array_element (Variables|Default|GetTrackList)
    (bind _returnvalue (Audio|CreateSound2D _array_element 1.0 1.0 0.0 0))
    (Utilities|Array|Add (Variables|Default|GetMusicRefs) _returnvalue)
    (Audio|Components|Audio|SetVolumeMultiplier _returnvalue 0.0 :!class /Script/Engine.AudioComponent)
    (Audio|Components|Audio|Play _returnvalue 0.0)
    (bind _foundwidgets (Widget|GetAllWidgetsOfClass "/Game/MainMenu/OptionsMenuWidget.OptionsMenuWidget_C" false)))
  (Audio|Components|Audio|SetVolumeMultiplier _output 1.0 :!class /Script/Engine.AudioComponent)
  (Variables|Default|SetCurrentMusicRef _output))

(fn ConstructionScript)