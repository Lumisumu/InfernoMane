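; MusicChangingVol_BP is a trigger volume that switches the background music when the player enters it.
; On BeginPlay it caches the first MusicManager_BP found in the level.
; When something overlaps its Box, it waits briefly, then, if that actor is the player character, tells the manager to change to the track index set in NextTrackToBePlayed.
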(event OnComponentBeginOverlap(Box)
  (params (OverlappedComponent :type Primitive%20Component%20Object%20Reference) (OtherActor :type Actor%20Object%20Reference) (OtherComp :type Primitive%20Component%20Object%20Reference) (OtherBodyIndex :type Integer) (bFromSweep :type Boolean) (SweepResult :type Hit%20Result%20Structure%20%28by%20ref%29))
  (Utilities|FlowControl|Delay 0.2)
  (if (== OtherActor (Game|GetPlayerCharacter 0))
    (Default|ChangeMusicto (Variables|Default|GetMusicManagerRef) (Variables|Default|GetNext%20track%20to%20be%20played) OtherActor)))

(event EventBeginPlay
  (bind _outactors (Actor|GetAllActorsOfClass "/Game/-Jason_TestiLevel/Blueprintit/MusicControlling/MusicManager_BP.MusicManager_BP_C"))
  (Variables|Default|SetMusicManagerRef (Utilities|Array|Get(acopy) _outactors)))

(event Collision|EventActorBeginOverlap
  (params (OtherActor :type Actor%20Object%20Reference)))

(event EventTick
  (params (DeltaSeconds :type Float%20%28single-precision%29)))

(fn ConstructionScript)