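; Ghost trail actor that leaves a frozen afterimage of the player's ThirdPersonCharacter, then fades and removes itself.
; On BeginPlay it gives each PoseableMesh material slot a dynamic fire material instance and copies the current pose from the player's mesh.
; An Opacity timeline is started to drive the Opacity parameter on those instances and destroy the actor when finished.
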(event Custom|GhostTrails
  (for _array_element (Rendering|Material|GetMaterials (Variables|Default|GetPoseableMesh))
    ;[1 1 1] Tässä voi (myös) vaihtaa trailin matskua
    (bind _returnvalue (Rendering|Material|CreateDynamicMaterialInstance "/Game/ASSETIT/HAHMOT/Yksisarvinen/materiaalit/mane/ALT_fire_Material_Inst.ALT_fire_Material_Inst" "None" "None" :!class /Script/Engine.KismetMaterialLibrary))
    (bind _returnvalue_2 (Utilities|Array|Add (Variables|Default|GetDynamicMats) _returnvalue))
    (Rendering|Material|SetMaterial (Variables|Default|GetPoseableMesh) _returnvalue_2 _returnvalue)
    (Class|PoseableMeshComponent|CopyPosefromSkeletalComponent (Variables|Default|GetPoseableMesh) (Variables|/Script/Engine.Character|GetMesh (Variables|Default|GetPlayerCharacterRef)))
    (Components|Timeline|PlayfromStart (Variables|Colors|GetOpacity))))

(event EventBeginPlay
  (bind _asthird_person_character (Utilities|Casting|CastToThirdPersonCharacter (Game|Player|GetPlayerPawn 0)))
  (Variables|Default|SetPlayerCharacterRef _asthird_person_character)
  (CallFunction|GhostTrails))

(fn ConstructionScript)